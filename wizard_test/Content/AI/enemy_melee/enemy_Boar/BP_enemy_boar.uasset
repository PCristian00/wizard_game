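; Boar melee enemy that damages BP_MainCharacter and reports its death to the room system.
; Incoming damage goes to TargetComponent, whose health drives a camera-facing health bar updated on Tick.
; Tick also checks AttackRange overlap, using a Delay to pace hits that land without rechecking range.
; On Destroyed, it finds the nearest RoomGenerator by 2D distance and calls UpdateRoomUponEnemyDeath to manage doors.
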(event EventDestroyed
  ;[0.15 0.15 0.15 0.5] Apertura porte
  (bind _outactors (Actor|GetAllActorsOfClass "/Script/wizard_test.RoomGenerator"))
  (bind _output_get (Variables|Default|SetroomGenerators _outactors))
  (bind _output_get_2 (Variables|Default|SetroomGenPos (Transformation|GetActorLocation (Utilities|Array|Get(acopy) _output_get))))
  (bind _output_get_3 (Variables|Default|SetenemyPos (Transformation|GetActorLocation)))
  (Variables|Default|SetshortestDistance (Math|Vector|Distance2D(Vector) _output_get_3 _output_get_2))
  (Variables|Default|SetclosestRoomGenIdx 0)
  (bind _result (Math|Integer|DecrementInt (Utilities|Array|Length (Variables|Default|GetroomGenerators)))
    (:%20%20
      (for _index (range 1 _result)
        ;;[0.15 0.15 0.15 0.5] Calcola la distanza tra il nemico distrutto e il "RoomGenerator" corrente al fine di trovare il "RoomGenerator" più vicino
        (bind _output_get_4 (Variables|Default|SetroomGenPos (Transformation|GetActorLocation (Utilities|Array|Get(acopy) (Variables|Default|GetroomGenerators) _index))))
        (bind _output_get_5 (Variables|Default|SetcurrentDistance (Math|Vector|Distance2D(Vector) _output_get_4 (Variables|Default|GetenemyPos))))
        (if (< _output_get_5 (Variables|Default|GetshortestDistance))
          (Variables|Default|SetshortestDistance _output_get_5)
          (Variables|Default|SetclosestRoomGenIdx _index)))
      ;;[0.15 0.15 0.15 0.5] Chiama la funzione del "RoomGenerator" per gestire le porte in base al numero dei nemici nella stanza
      (bind _asroom_generator (Utilities|Casting|CastToRoomGenerator (Utilities|Array|Get(acopy) (Variables|Default|GetroomGenerators) (Variables|Default|GetclosestRoomGenIdx))))
      (bind _output_get_6 (Variables|Default|SetnearestRoomGen _asroom_generator))
      (Class|RoomGenerator|UpdateRoomUponEnemyDeath _output_get_6))))

(event Game|Damage|EventAnyDamage
  (params (Damage :type Float%20%28single-precision%29) (DamageType :type Damage%20Type%20Object%20Reference) (InstigatedBy :type Controller%20Object%20Reference) (DamageCauser :type Actor%20Object%20Reference))
  ;[0.15 0.15 0.15 0.5] Nemico prende danno
  (Default|TargetDamage (Variables|Default|GetTargetComponent) Damage DamageType))

(event EventTick
  (params (DeltaSeconds :type Float%20%28single-precision%29))
  (bind _healthbar_widget (Variables|Default|GetHealthBar%20Widget))
  ;[0.15 0.15 0.15 0.5] Barra della vita
  (bind _aswb_enemy_health (Utilities|Casting|CastToWB_EnemyHealth (UserInterface|GetWidget (Variables|Default|GetHealthBar%20Widget))))
  (bind _health (Default|GetHealth (Variables|Default|GetTargetComponent)))
  (Progress|SetPercent (Variables|/Game/AI/WB_EnemyHealth.WB_EnemyHealth_C|GetHealthBar_Enemy _aswb_enemy_health) (/ _health (Variables|Default|GetMaxHealth)))
  (Transformation|SetWorldRotation _healthbar_widget (Math|Rotator|FindLookatRotation (Transformation|GetWorldLocation _healthbar_widget) (Transformation|GetWorldLocation (Variables|/Script/Engine.PlayerCameraManager|GetTransformComponent (Game|GetPlayerCameraManager 0)))) false false)
  ;[0.15 0.15 0.15 0.5] Nemico fa danno
  (bind _returnvalue (Actor|GetActorOfClass "/Game/Dragos/Blueprint/BP_MainCharacter.BP_MainCharacter_C"))
  (if (Collision|IsOverlappingActor (Variables|Default|GetAttackRange) _returnvalue :!class /Script/Engine.PrimitiveComponent)
    (Utilities|FlowControl|Delay 0.9)
    (Game|Damage|ApplyDamage _returnvalue 5.0 0 0)))

(fn ConstructionScript)