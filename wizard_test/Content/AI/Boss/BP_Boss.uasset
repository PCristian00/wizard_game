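; Boss enemy character with a melee attack, an on-screen health bar and a death that ends the game in victory.
; Attack plays a montage whose notify sphere-traces at a finger socket and damages BP_MainCharacter, with a flag blocking overlapping swings.
; AnyDamage feeds TargetComponent, whose health Tick polls to update the bar.
; At zero health it plays a death montage, then after a delay shows the victory menu and pauses the game.
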(event EventBeginPlay
  (bind _returnvalue (UserInterface|CreateWidget "/Game/AI/Boss/WB_BossHealth.WB_BossHealth_C"))
  (UserInterface|Viewport|AddtoViewport _returnvalue 0)
  (Variables|Default|Sethealth_UI _returnvalue))

(event EventTick
  (params (DeltaSeconds :type Float%20%28single-precision%29))
  (bind _returnvalue (Game|GetPlayerController 0))
  ;[0.15 0.15 0.15 0.5] Gestione della vita del boss
  (bind _health (Default|GetHealth (Variables|Default|GetTargetComponent)))
  (Progress|SetPercent (Variables|/Game/AI/Boss/WB_BossHealth.WB_BossHealth_C|GetHealthBar (Variables|Default|Gethealth_UI)) (/ _health (Variables|Default|GetMaxHealth)))
  (if (<= _health 0.0)
    (if (not (Variables|Default|GetIsDeath))
      (Variables|Default|SetIsDeath true)
      (Pawn|Components|CharacterMovement|DisableMovement (Variables|Character|GetCharacterMovement))
      (Animation|PlayAnimMontage "/Game/AI/Boss/Animations/Death_Montage.Death_Montage" 1.0 "None")
      (Utilities|FlowControl|Delay 7.0)
      (bind _returnvalue_2 (UserInterface|CreateWidget "/Game/UI/WB_VictoryMenu.WB_VictoryMenu_C"))
      (UserInterface|Viewport|AddtoViewport _returnvalue_2 0)
      (Variables|/Script/Engine.PlayerController|SetbShowMouseCursor _returnvalue true)
      (Input|SetInputModeUIOnly _returnvalue 0 "DoNotLock" false)
      (Game|SetGamePaused true))))

(event EventAttack
  (bind _mesh (Variables|Character|GetMesh))
  (bind _returnvalue (Transformation|GetSocketLocation _mesh "Bip001-R-Finger21"))
  ;[0.15 0.15 0.15 0.5] Attacco melee del boss
  (if (not (Variables|Default|GetisAttacking))
    (Animation|Montage|PlayMontage (Variables|Character|GetMesh) "/Game/AI/Boss/Animations/MeleeAttack_Montage.MeleeAttack_Montage"
      (:then
        (Variables|Default|SetisAttacking true))
      (:OnCompleted
        (Variables|Default|SetisAttacking false))
      (:OnNotifyBegin
        (bind _outhit (Collision|SphereTraceForObjects _returnvalue _returnvalue 5e+01 (Utilities|Array|MakeArray "ObjectTypeQuery3") false 0 "None"))
        (bind _asbp_main_character (Utilities|Casting|CastToBP_MainCharacter (.HitActor (Collision|BreakHitResult _outhit))))
        (Game|Damage|ApplyDamage _asbp_main_character 25.0 0 0)))))

(event Game|Damage|EventAnyDamage
  (params (Damage :type Float%20%28single-precision%29) (DamageType :type Damage%20Type%20Object%20Reference) (InstigatedBy :type Controller%20Object%20Reference) (DamageCauser :type Actor%20Object%20Reference))
  ;[0.15 0.15 0.15 0.5] Nemico prende danno
  (Default|TargetDamage (Variables|Default|GetTargetComponent) Damage DamageType false))

(fn ConstructionScript)