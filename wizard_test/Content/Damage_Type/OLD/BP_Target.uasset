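; BP_Target is a damageable target actor that tracks Health and destroys itself when Health reaches zero or below.
; AnyDamage passes base DamageType hits straight to UpdateHealth.
; Other damage types get the StatusEffectComponent through an interface message, which returns adjusted damage, status effect and critical-hit flag before UpdateHealth runs.
; Each step prints timestamped debug text, partly in Italian, and an invalid component prints an error without applying damage.
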(event Game|Damage|EventAnyDamage
  (params (Damage :type Float%20%28single-precision%29) (DamageType :type Damage%20Type%20Object%20Reference) (InstigatedBy :type Controller%20Object%20Reference) (DamageCauser :type Actor%20Object%20Reference))
  (bind _statuseffectcomponent (Variables|Default|GetStatusEffectComponent))
  (if (== (Utilities|GetClass DamageType) "/Script/Engine.DamageType")
    (Development|PrintString "Danno normale")
    (CallFunction|UpdateHealth Damage)
    (Development|PrintText (Utilities|Text|FormatText "BPT {time}> DMG: {dmg} HEALTH: {health}" (Class|KismetTextLibrary|AsTimeDateTime (Math|DateTime|UTCNow)) Damage (Variables|Default|GetHealth)) true true "(R=0.715221,G=0.739583,B=0.732098,A=1.000000)")
    (else
      (Utilities|IsValid _statuseffectcomponent
        (:Is%20Valid
          (bind (_statuseffect _adjusteddamage _criticalhit) (Class|DamageTypeInterface|TriggerEffectInterface(Message) DamageType _statuseffectcomponent Damage))
          (CallFunction|UpdateHealth _adjusteddamage)
          (Development|PrintText (Utilities|Text|FormatText "BPT {time}> DMG: {dmg}   TYPE: {statusEffect}   CRIT: {isCrit} HEALTH: {health}" (Class|KismetTextLibrary|AsTimeDateTime (Math|DateTime|UTCNow)) _adjusteddamage (|GenerictoText _statuseffect) _criticalhit (Variables|Default|GetHealth)) true true "(R=0.715221,G=0.739583,B=0.732098,A=1.000000)"))
        (:Is%20Not%20Valid
          (Development|PrintText "SSE non valido"))))))

(fn ConstructionScript)

(fn UpdateHealth
  (params (Damage :type Float%20%28double-precision%29))
  (bind _self self)
  (bind _returnvalue (Utilities|GetDisplayName _self))
  (if (!= Damage 0.0)
    (Development|PrintText (Utilities|Text|FormatText "UH {time}: {target} ha subito {damage} danni." (Class|KismetTextLibrary|AsTimeDateTime (Math|DateTime|UTCNow)) _returnvalue Damage))
    (bind _output_get (Variables|Default|SetHealth (- (Variables|Default|GetHealth) Damage)))
    (if (<= _output_get 0)
      (Actor|DestroyActor)
      (Development|PrintText (Utilities|Text|FormatText "{name} distrutto." _returnvalue) true true "(R=1.000000,G=0.067295,B=0.000000,A=1.000000)" 5.0))
    (else
      (Development|PrintText "UH Nessun danno"))))