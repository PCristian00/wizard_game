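; BP_IceHoming is an ice homing projectile actor with a Sphere collision body.
; On hit, the Sphere passes the other actor to HomingComponent's CheckTarget, then to ProjectileComponent's hit handler with radial damage off.
; Find Homing Target searches actors tagged "Homing", excludes the projectile's owner, and returns a SceneComponent from the nearest one.
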(event OnComponentHit(Sphere)
  (params (HitComponent :type Primitive%20Component%20Object%20Reference) (OtherActor :type Actor%20Object%20Reference) (OtherComp :type Primitive%20Component%20Object%20Reference) (NormalImpulse :type Vector :default "0, 0, 0") (Hit :type Hit%20Result%20Structure%20%28by%20ref%29))
  (Default|CheckTarget (Variables|Default|GetHomingComponent) (Variables|Default|GetSphere) OtherActor)
  (Default|OnComponentHit (Variables|Default|GetProjectileComponent) OtherActor false))

(fn ConstructionScript)

(fn FindHomingTarget
  (bind _outactors (Actor|GetAllActorsOfClasswithTag "/Script/Engine.Actor" "Homing"))
  (Utilities|Array|RemoveItem _outactors (Components|GetOwner))
  (Utilities|IsValid (.ReturnValue (Actor|FindNearestActor (Transformation|GetActorLocation) _outactors))
    (:Is%20Valid
      (return (Actor|GetComponentbyClass (.ReturnValue (Actor|FindNearestActor (Transformation|GetActorLocation) _outactors)) "/Script/Engine.SceneComponent")))
    (:Is%20Not%20Valid
      (return 0))))