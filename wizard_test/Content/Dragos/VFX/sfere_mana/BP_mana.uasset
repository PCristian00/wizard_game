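; Mana orb pickup that homes in on the player and restores mana.
; On BeginPlay, it sets the first BP_MainCharacter's root as the ProjectileMovement homing target.
; On overlap, it compares the other actor's class to that character instance; a match adds ManaAddingValue to ShooterComponent mana, plays a sound and destroys the orb.
; Overflow past MaxMana sets mana to a hardcoded 100 instead of MaxMana.
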(event EventBeginPlay
  (bind _outactors (Actor|GetAllActorsOfClass "/Game/Dragos/Blueprint/BP_MainCharacter.BP_MainCharacter_C"))
  (bind _output_get (Variables|Default|SetPlayerCharacter (Utilities|Array|Get(acopy) _outactors)))
  (Variables|/Script/Engine.ProjectileMovementComponent|SetHomingTargetComponent (Variables|Default|GetProjectileMovement) (Variables|/Script/Engine.Actor|GetRootComponent _output_get)))

(event Collision|EventActorBeginOverlap
  (params (OtherActor :type Actor%20Object%20Reference))
  (bind _outactors (Actor|GetAllActorsOfClass "/Game/Dragos/Blueprint/BP_MainCharacter.BP_MainCharacter_C"))
  (if (== (Utilities|GetClass OtherActor) (Utilities|Array|Get(acopy) _outactors))
    (if (> (+ (Variables|/Game/Damage_Type/ShooterComponent.ShooterComponent_C|GetMana (Variables|/Game/Dragos/Blueprint/BP_MainCharacter.BP_MainCharacter_C|GetShooterComponent (Utilities|Array|Get(acopy) _outactors))) (Variables|Default|GetManaAddingValue)) (Variables|/Game/Damage_Type/ShooterComponent.ShooterComponent_C|GetmaxMana (Variables|/Game/Dragos/Blueprint/BP_MainCharacter.BP_MainCharacter_C|GetShooterComponent (Utilities|Array|Get(acopy) _outactors))))
      (Variables|/Game/Damage_Type/ShooterComponent.ShooterComponent_C|SetMana (Variables|/Game/Dragos/Blueprint/BP_MainCharacter.BP_MainCharacter_C|GetShooterComponent (Utilities|Array|Get(acopy) _outactors)) 1e+02)
      (else
        (Variables|/Game/Damage_Type/ShooterComponent.ShooterComponent_C|SetMana (Variables|/Game/Dragos/Blueprint/BP_MainCharacter.BP_MainCharacter_C|GetShooterComponent (Utilities|Array|Get(acopy) _outactors)) (+ (Variables|/Game/Damage_Type/ShooterComponent.ShooterComponent_C|GetMana (Variables|/Game/Dragos/Blueprint/BP_MainCharacter.BP_MainCharacter_C|GetShooterComponent (Utilities|Array|Get(acopy) _outactors))) (Variables|Default|GetManaAddingValue)))))
    (Audio|PlaySound2D "/Game/PowerUp/Sound/S_mana.S_mana" 1.0 1.0 0.0 0 0)
    (Actor|DestroyActor)))

(fn ConstructionScript)