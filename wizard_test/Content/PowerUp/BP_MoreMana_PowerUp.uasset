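; BP_MoreMana_PowerUp is a pickup that permanently raises the player's mana capacity.
; When an overlapping actor casts to BP_MainCharacter, it adds IncreaseValue to both MaxMana and current Mana on that character's ShooterComponent.
; It then plays a 2D mana sound and destroys itself, so each pickup works once.
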(event Collision|EventActorBeginOverlap
  (params (OtherActor :type Actor%20Object%20Reference))
  (bind _increasevalue (Variables|Default|GetIncreaseValue))
  (bind _asbp_main_character (Utilities|Casting|CastToBP_MainCharacter OtherActor))
  (Variables|/Game/Damage_Type/ShooterComponent.ShooterComponent_C|SetmaxMana (Variables|/Game/Dragos/Blueprint/BP_MainCharacter.BP_MainCharacter_C|GetShooterComponent _asbp_main_character) (+ (Variables|/Game/Damage_Type/ShooterComponent.ShooterComponent_C|GetmaxMana (Variables|/Game/Dragos/Blueprint/BP_MainCharacter.BP_MainCharacter_C|GetShooterComponent _asbp_main_character)) _increasevalue))
  (Variables|/Game/Damage_Type/ShooterComponent.ShooterComponent_C|SetMana (Variables|/Game/Dragos/Blueprint/BP_MainCharacter.BP_MainCharacter_C|GetShooterComponent _asbp_main_character) (+ (Variables|/Game/Damage_Type/ShooterComponent.ShooterComponent_C|GetMana (Variables|/Game/Dragos/Blueprint/BP_MainCharacter.BP_MainCharacter_C|GetShooterComponent _asbp_main_character)) _increasevalue))
  (Audio|PlaySound2D "/Game/PowerUp/Sound/S_mana.S_mana" 1.0 1.0 0.0 0 0)
  (Actor|DestroyActor))

(fn ConstructionScript)